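; BP_HealthPack is a health pickup that restores a small amount of health to the player.
; A component hit on the HealthPack component casts to BP_Player, sets Used, adds to HealthValue with a cap at 100, then destroys the actor.
; Tick also destroys the pack once game time passes a fixed lifetime after TimeCreated, which is not assigned in these graphs.
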(event OnComponentHit(HealthPack)
  (params (HitComponent :type Primitive%20Component%20Object%20Reference) (OtherActor :type Actor%20Object%20Reference) (OtherComp :type Primitive%20Component%20Object%20Reference) (NormalImpulse :type Vector :default "0, 0, 0") (Hit :type Hit%20Result%20Structure%20%28by%20ref%29))
  (bind _asbp_player (Utilities|Casting|CastToBP_Player OtherActor))
  (Variables|Default|SetUsed true)
  (if (<= (Variables|/Game/InfiniteMatrix/Blueprints/BP_Player.BP_Player_C|GetHealthValue _asbp_player) 95)
    (Variables|/Game/InfiniteMatrix/Blueprints/BP_Player.BP_Player_C|SetHealthValue _asbp_player (+ (Variables|/Game/InfiniteMatrix/Blueprints/BP_Player.BP_Player_C|GetHealthValue _asbp_player) 5))
    (else
      (Variables|/Game/InfiniteMatrix/Blueprints/BP_Player.BP_Player_C|SetHealthValue _asbp_player (+ (Variables|/Game/InfiniteMatrix/Blueprints/BP_Player.BP_Player_C|GetHealthValue _asbp_player) (- 100 (Variables|/Game/InfiniteMatrix/Blueprints/BP_Player.BP_Player_C|GetHealthValue _asbp_player))))))
  (Actor|DestroyActor))

(event EventBeginPlay)

(event Collision|EventActorBeginOverlap
  (params (OtherActor :type Actor%20Object%20Reference)))

(event EventTick
  (params (DeltaSeconds :type Float%20%28single-precision%29))
  (if (>= (Utilities|Time|GetTimeSeconds) (+ (Variables|Default|GetTimeCreated) 20))
    (Actor|DestroyActor)))

(fn ConstructionScript)