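; BP_Enemy is an enemy actor that hurts the player on contact and awards score when hit by a projectile.
; Overlapping BP_Player triggers red haze and health loss, and a fatal hit shows restart and destroys the enemy.
; A BP_Projectile overlap destroys both actors and raises the player's score.
; Tick also destroys the enemy once a fixed lifetime past TimeMade elapses.
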(event EventBeginPlay)

(event Collision|EventActorBeginOverlap
  (params (OtherActor :type Actor%20Object%20Reference))
  (bind _asbp_player (Utilities|Casting|CastToBP_Player OtherActor)
    (:then
      (Default|DisplayRedHaze _asbp_player)
      (Default|LowerHealth _asbp_player 5)
      (if (Variables|/Game/InfiniteMatrix/Blueprints/BP_Player.BP_Player_C|GetIsDead _asbp_player)
        (Default|DisplayRestart _asbp_player)
        (Actor|DestroyActor :!label _label)))
    (:CastFailed
      (bind _asbp_player_2 (Utilities|Casting|CastToBP_Player (Game|Player|GetPlayerPawn 0)))
      (bind _asbp_projectile (Utilities|Casting|CastToBP_Projectile OtherActor))
      (Actor|DestroyActor _asbp_projectile)
      (Default|ChangeScore _asbp_player_2 2e+01)
      (goto _label))))

(event EventTick
  (params (DeltaSeconds :type Float%20%28single-precision%29))
  (if (>= (Utilities|Time|GetTimeSeconds) (+ (Variables|Default|GetTimeMade) 15))
    (Actor|DestroyActor)))

(fn ConstructionScript)