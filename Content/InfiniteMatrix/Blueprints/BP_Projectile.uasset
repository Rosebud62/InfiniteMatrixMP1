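; BP_Projectile is a projectile actor that travels along world X and destroys itself when its ProjectileShape component begins an overlap.
; Each Tick it casts player pawn 0 to BP_Player and offsets itself by three times that player's current ForwardSpeed, scaled by delta time.
; A two-second lifetime check destroys it only when game time exactly equals TimeAtSpawn plus two, and TimeAtSpawn is not set in these graphs.
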(event OnComponentBeginOverlap(ProjectileShape)
  (params (OverlappedComponent :type Primitive%20Component%20Object%20Reference) (OtherActor :type Actor%20Object%20Reference) (OtherComp :type Primitive%20Component%20Object%20Reference) (OtherBodyIndex :type Integer) (bFromSweep :type Boolean) (SweepResult :type Hit%20Result%20Structure%20%28by%20ref%29))
  (Actor|DestroyActor))

(event EventBeginPlay)

(event EventTick
  (params (DeltaSeconds :type Float%20%28single-precision%29))
  (if (== (+ (Variables|Default|GetTimeAtSpawn) 2.0) (Utilities|Time|GetTimeSeconds))
    (Actor|DestroyActor)
    (else
      (bind _asbp_player (Utilities|Casting|CastToBP_Player (Game|Player|GetPlayerPawn 0)))
      (Transformation|AddActorWorldOffset (Math|Vector|MakeVector (* DeltaSeconds (* (Variables|/Game/InfiniteMatrix/Blueprints/BP_Player.BP_Player_C|GetForwardSpeed _asbp_player) 3.0)) 0.0 0.0)))))

(fn ConstructionScript)